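; Flappy Bird pipe obstacle that scores the bird's passes and ends the game on pipe contact.
; The construction script randomizes its vertical offset.
; Box overlap increments the bird's score, updates the score widget and, at set milestones, plays a point sound and tells the spawner to decrease its timer.
; Pipe overlaps trigger Death, which pauses the game, shows the game-over UI and checks and displays the saved highscore.
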(event `self.ReceiveBeginPlay`
  (bind _returnvalue (`GameplayStatics.GetActorOfClass` "/Game/Flappybird/BluePrints/BP_Bird.BP_Bird_C"))
  (set `self.BP_BirdREF` _returnvalue)
  (bind _returnvalue_2 (`GameplayStatics.GetActorOfClass` "/Game/Flappybird/BluePrints/BP_Obstaclesspawner.BP_Obstaclesspawner_C"))
  (set `self.BP_ObstaclesSpawnerREF` _returnvalue_2))

(event `self.Box.OnComponentBeginOverlap`
  (params (OverlappedComponent :type "PrimitiveComponent Object Reference") (OtherActor :type "Actor Object Reference") (OtherComp :type "PrimitiveComponent Object Reference") (OtherBodyIndex :type Integer) (bFromSweep :type Boolean) (SweepResult :type "HitResult Structure (by ref)"))
  (if (== OtherActor (`self.BP_BirdREF`))
    (`GameplayStatics.PlaySound2D` "/Game/Flappybird/Audio/Flap.Flap" 1.0 1.0 0.0 null null)
    (bind _output_get (`/Game/Flappybird/BluePrints/BP_Bird.UpdateScore` (`self.BP_BirdREF`)))
    (bind _foundwidgets (`WidgetBlueprintLibrary.GetAllWidgetsOfClass` "/Game/Flappybird/UMG/WBP_Score.WBP_Score_C"))
    (message `/Game/Flappybird/BluePrints/Interface/IF_Score.SetScore` (`|GetArrayItem` _foundwidgets) (`KismetTextLibrary.Conv_IntToText` _output_get))
    ;[0.09896 0.06554 0] Branch
    (if (== (`/Game/Flappybird/BluePrints/BP_Bird.Score` (`self.BP_BirdREF`)) 2)
      (`GameplayStatics.PlaySound2D` "/Game/Flappybird/Audio/Point.Point" 1.0 1.0 0.0 null null)
      (message `/Game/Flappybird/BluePrints/Interface/IF_ObstaclesSpeed.Decrease Timer` (`self.BP_ObstaclesSpawnerREF`) :!label _label)
      (elif (== (`/Game/Flappybird/BluePrints/BP_Bird.Score` (`self.BP_BirdREF`)) 5)
        (`GameplayStatics.PlaySound2D` "/Game/Flappybird/Audio/Point.Point" 1.0 1.0 0.0 null null)
        (goto _label)
        (elif (== (`/Game/Flappybird/BluePrints/BP_Bird.Score` (`self.BP_BirdREF`)) 8)
          (`GameplayStatics.PlaySound2D` "/Game/Flappybird/Audio/Point.Point" 1.0 1.0 0.0 null null)
          (goto _label))))))

(event `Death`
  (bind _returnvalue (`GameplayStatics.GetPlayerController` 0))
  (`GameplayStatics.PlaySound2D` "/Game/Flappybird/Audio/Die.Die" 1.0 1.0 0.0 null null)
  (`GameplayStatics.SetGamePaused` true)
  (bind _returnvalue_2 (`|CreateWidget` "/Game/Flappybird/UMG/WBP_GameOver.WBP_GameOver_C" (`GameplayStatics.GetPlayerController` 0)))
  (bind _output_get (set `self.WB_GameOverREF` _returnvalue_2))
  (`UserWidget.AddToViewport` _output_get 0)
  (set `PlayerController.bShowMouseCursor` true _returnvalue)
  (`WidgetBlueprintLibrary.SetInputMode_UIOnlyEx` _returnvalue null)
  (message `/Game/Flappybird/BluePrints/Interface/IF_Highscore.Is Highscore?` (`self.BP_BirdREF`))
  (`/Game/Flappybird/UMG/WBP_GameOver.ShowScores` (`self.WB_GameOverREF`) (`KismetTextLibrary.Conv_IntToText` (`/Game/Flappybird/BluePrints/SG_Highscore.SaveScore` (`/Game/Flappybird/BluePrints/BP_Bird. Highscore Save REF` (`self.BP_BirdREF`))))))

(event `self.UpperPipe.OnComponentBeginOverlap`
  (params (OverlappedComponent :type "PrimitiveComponent Object Reference") (OtherActor :type "Actor Object Reference") (OtherComp :type "PrimitiveComponent Object Reference") (OtherBodyIndex :type Integer) (bFromSweep :type Boolean) (SweepResult :type "HitResult Structure (by ref)"))
  (if (== OtherActor (`self.BP_BirdREF`))
    (`self.Death`)))

(event `self.Lowerpipe.OnComponentBeginOverlap`
  (params (OverlappedComponent :type "PrimitiveComponent Object Reference") (OtherActor :type "Actor Object Reference") (OtherComp :type "PrimitiveComponent Object Reference") (OtherBodyIndex :type Integer) (bFromSweep :type Boolean) (SweepResult :type "HitResult Structure (by ref)"))
  (if (== OtherActor (`self.BP_BirdREF`))
    (`self.Death`)))

(fn `UserConstructionScript`
  (`SceneComponent.K2_AddLocalOffset` (`self.DefaultSceneRoot`) (`KismetMathLibrary.MakeVector` 0.0 0.0 (`KismetMathLibrary.RandomFloatInRange` -100.0 150.0)) false false))
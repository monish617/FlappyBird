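; Player pawn for a Flappy Bird minigame that turns the flap input into jumps for the bird actor in the level.
; On BeginPlay it adds the Flappy Enhanced Input mapping context, caches the placed BP_Bird and creates the score widget on screen.
; Each flap press overwrites the bird sphere's physics linear velocity with an upward jump speed, so the pawn controls a separate physics-driven bird.
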(event `self.ReceiveBeginPlay`
  (`|ExecutionSequence`
    (:`then_0`
      (bind _asplayer_controller (cast `PlayerController` (`self.GetController`)))
      (bind _returnvalue (pcsubsystem `EnhancedInputLocalPlayerSubsystem` _asplayer_controller))
      (`/Engine/EditorBlueprintResources/StandardMacros.IsValid` _returnvalue
        (:`Is Valid`
          (`EnhancedInputSubsystemInterface.AddMappingContext` _returnvalue "/Game/Flappybird/Input/IMC_Flappy.IMC_Flappy" 0 (struct)))))
    (:`then_1`
      (bind _returnvalue_2 (`GameplayStatics.GetActorOfClass` "/Game/Flappybird/BluePrints/BP_Bird.BP_Bird_C"))
      (set `self.BP_Bird_REF` _returnvalue_2)
      (bind _returnvalue_3 (`|CreateWidget` "/Game/Flappybird/UMG/WBP_Score.WBP_Score_C" (`GameplayStatics.GetPlayerController` 0)))
      (`UserWidget.AddToViewport` _returnvalue_3 0))))

(event `EnhancedInput|/Game/Flappybird/Input/IA_Flap`
  (params (ActionValue :type Boolean) (ElapsedSeconds :type "Float (double-precision)") (TriggeredSeconds :type "Float (double-precision)") (InputAction :type "InputAction Object Reference" :default "/Game/Flappybird/Input/IA_Flap.IA_Flap"))
  (:`Started`
    (`PrimitiveComponent.SetPhysicsLinearVelocity` (`/Game/Flappybird/BluePrints/BP_Bird.Sphere` (`self.BP_Bird_REF`)) (`KismetMathLibrary.MakeVector` 0.0 0.0 (`self.JumpSpeed`)) false "None")))

(fn `UserConstructionScript`)
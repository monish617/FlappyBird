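; BP_Obstaclesspawner spawns BP_Obstacle actors at a fixed location for the Flappy Bird game, starting on BeginPlay.
; Each Spawn re-arms a one-shot timer using the Time variable, forming a repeating loop, and prints that interval for debugging.
; DecreaseTimer lowers Time by one second to shorten later spawn intervals; IncreaseObstaclesSpeed is an empty stub.
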(event `self.ReceiveBeginPlay`
  (`self.Spawn`))

(event `Spawn`
  (bind _time (`self.Time`))
  (`|SpawnActorFromClass` "/Game/Flappybird/BluePrints/BP_Obstacle.BP_Obstacle_C" (`KismetMathLibrary.MakeTransform` (0.0 700.0 -200.0)) "Undefined" "MultiplyWithRoot" null null)
  (`KismetSystemLibrary.K2_SetTimerDelegate` (delegate `Spawn`) _time)
  (`KismetSystemLibrary.PrintString` (`KismetStringLibrary.Conv_DoubleToString` _time)))

(event `/Game/Flappybird/BluePrints/Interface/IF_ObstaclesSpeed.Decrease Timer`
  (set `self.Time` (- (`self.Time`) 1.0)))

(fn `Increase obstacles speed`)

(fn `UserConstructionScript`)
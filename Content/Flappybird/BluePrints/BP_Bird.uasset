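; BP_Bird is the Flappy Bird game's bird Blueprint, and its graphs handle scoring and high score persistence.
; On BeginPlay it loads the SG_Highscore save from its slot, or creates and saves a new one if none exists.
; UpdateScore adds Scoretoadd to the running score and returns it.
; The IsHighscore? event writes the score to the save slot when it beats the stored best.
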(event `self.ReceiveBeginPlay`
  (bind _returnvalue (`GameplayStatics.DoesSaveGameExist` (`self.Slot Name`)))
  (if _returnvalue
    (bind _returnvalue_2 (`GameplayStatics.LoadGameFromSlot` (`self.Slot Name`)))
    (bind _ashighscore_save (cast `/Game/Flappybird/BluePrints/SG_Highscore` _returnvalue_2))
    (set `self. Highscore Save REF` _ashighscore_save)
    (else
      (bind _returnvalue_3 (`GameplayStatics.CreateSaveGameObject` "/Game/Flappybird/BluePrints/SG_Highscore.SG_Highscore_C"))
      (bind _output_get (set `self. Highscore Save REF` _returnvalue_3))
      (`GameplayStatics.SaveGameToSlot` _output_get (`self.Slot Name`)))))

(event `/Game/Flappybird/BluePrints/Interface/IF_Highscore.Is Highscore?`
  (bind __highscore_save_ref (`self. Highscore Save REF`))
  (if (> (`self.Score`) (`/Game/Flappybird/BluePrints/SG_Highscore.SaveScore` (`self. Highscore Save REF`)))
    (set `/Game/Flappybird/BluePrints/SG_Highscore.SaveScore` (`self.Score`) __highscore_save_ref)
    (`GameplayStatics.SaveGameToSlot` __highscore_save_ref (`self.Slot Name`))))

(fn `UpdateScore`
  (returns (Output_Get :type Integer))
  (bind _output_get (set `self.Score` (+ (`self.Score`) (`self.scoretoadd`))))
  (return _output_get))

(fn `UserConstructionScript`)